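; BP_Cube is a damageable cube actor that destroys itself when its health runs out.
; AnyDamage subtracts damage from CurrentHealth, broadcasts the new value through the HitDamage dispatcher, then destroys the actor at zero or below.
; Separately, pressing the 3 key sets the static mesh's relative location to a fixed X offset, and releasing it prints a test string.
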(event `self.ReceiveAnyDamage`
  (params (Damage :type "Float (single-precision)") (DamageType :type "DamageType Object Reference") (InstigatedBy :type "Controller Object Reference") (DamageCauser :type "Actor Object Reference"))
  (bind _output_get (set `self.CurrentHealth` (- (`self.CurrentHealth`) Damage)))
  (`self.HitDamage` _output_get)
  (if (<= _output_get 0.0)
    (`self.K2_DestroyActor`)))

(event `Key|Three`
  (params (Key :type "Key Structure"))
  (:`Pressed`
    (`SceneComponent.K2_SetRelativeLocation` (`self.StaticMeshComponent0`) (200.0 0.0 0.0) false false))
  (:`Released`
    (`KismetSystemLibrary.PrintString` "Hello")))

(fn `UserConstructionScript`)